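; GI_Tutorial is a Game Instance that shows the player's in-game status through Discord Rich Presence.
; On Init it creates and initializes a DiscordRpc object with the application ID, then publishes a default status.
; A RichPresence function writes state, details and start timestamp, ignoring its image key input, then pushes the update, and a second Rich Presence function wraps it.
; Shutdown clears the presence.
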(event EventInit
  (bind _returnvalue (Game|ConstructObjectfromClass "/Script/DiscordRpc.DiscordRpc"))
  (bind _output_get (Variables|Discord|SetDiscordRPC _returnvalue))
  (Class|DiscordRpc|Initialize _output_get (Variables|Discord|GetApplication%20Id) false)
  (Discord|RichPresence "In game" "Currently in game "))

(event EventShutdown
  (Class|DiscordRpc|ClearPresence (Variables|Discord|GetDiscordRPC)))

(fn RichPresence
  (params (State :type String) (Details :type String) (Start%20Timestamp :type Integer) (Large%20Image%20Key :type Image%20Soft%20Class%20Reference))
  (bind _discordrpc (Variables|Discord|GetDiscordRPC))
  (bind _structout (Utilities|Struct|SetmembersinDiscordRichPresence (Variables|/Script/DiscordRpc.DiscordRpc|GetRichPresence (Variables|Discord|GetDiscordRPC)) State Details Start%20Timestamp))
  (Variables|/Script/DiscordRpc.DiscordRpc|SetRichPresence _discordrpc _structout)
  (Class|DiscordRpc|UpdatePresence _discordrpc)
  (return true))

(fn RichPresence
  (params (State :type String) (Details :type String))
  (bind _return_value (Discord|RichPresence State Details))
  (return _return_value))